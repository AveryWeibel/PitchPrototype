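; Blood spray effect actor that animates a blood material on a plane, then removes itself.
; On BeginPlay it creates a dynamic instance of BloodPlane_Inst and applies it to the plane.
; After a short delay, a timeline drives the material's SprayProgress parameter, and the actor destroys itself when it finishes.
; An unconnected HueShift parameter update is left unused in the graph.
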(event EventBeginPlay
  (bind _returnvalue (Rendering|Material|CreateDynamicMaterialInstance "/Game/myVFX/myMaterials/BloodPlane_Inst.BloodPlane_Inst" "None" "None" :!class /Script/Engine.KismetMaterialLibrary))
  (bind _output_get (Variables|Default|SetBloodMat _returnvalue))
  (Rendering|Material|SetMaterial (Variables|Default|GetPlane) 0 _output_get)
  (Utilities|FlowControl|Delay 5.0)
  (bind _newtrack_0 (Timeline|BloodTImeline Play)
    (:Update
      (Rendering|Material|SetScalarParameterValue (Variables|Default|GetBloodMat) "SprayProgress" _newtrack_0 :!class /Script/Engine.MaterialInstanceDynamic))
    (:Finished
      (Actor|DestroyActor))))

(fn ConstructionScript)