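; Sundial actor that plays the visual, audio and camera effects for the staged apocalypse sequence.
; BeginPlay creates dynamic materials for the dial, water and light beams, then registers a callback on Ocean2_Blueprint that binds Stage0–3 to ApocManager's stage events.
; Each stage's timeline drives material and particle parameters for water glow, bubbles and the light geyser.
; Stage 2 adds distance-scaled camera shake; Stage 3 also widens the inner beam.
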(event Custom|Stage0
  ;[1 1 1] Stage 0
  (bind _brightnesstrack (Timeline|Stage0_TL Play)
    (:Update
      (Rendering|Material|SetScalarParameterValue (Variables|Default|GetSundialWaterMat) "DimensionMix" (* _brightnesstrack 1e+01) :!class /Script/Engine.MaterialInstanceDynamic)
      (Effects|Components|ParticleSystem|SetFloatParameter (Variables|Default|GetParts_Beam) "FloatingSpawn" (* _brightnesstrack 2e+02)))))

(event Custom|Stage2
  (Effects|Components|ParticleSystem|SetFloatParameter (Variables|Components|GetParts_Bubs) "BubbleSpawn" 0.0)
  (Audio|SpawnSoundatLocation "/Game/myVFX/Apocalypse/Rumbling.Rumbling" (Transformation|GetWorldLocation (Variables|Default|GetDefaultSceneRoot)) "0, 0, 0" 1.8 1.0 0.0 "/Game/myVFX/Apocalypse/RumblingAttenuation_2.RumblingAttenuation_2" 0)
  (bind _apoc2_track (Timeline|Stage2_TL Play)
    (:Update
      (Effects|Components|ParticleSystem|SetFloatParameter (Variables|Default|GetParts_Beam) "RibbonSpawn" (+ (* _apoc2_track 3e+02) 2e+02))
      (Rendering|Material|SetScalarParameterValue (Variables|Default|GetBeamMat) "OpacOffset" (- 1.5 (/ _apoc2_track 8.0)) :!class /Script/Engine.MaterialInstanceDynamic)
      (Rendering|Material|SetScalarParameterValue (Variables|Default|GetLightGeyserInnerMat) "OpacOffset" (- 1.5 (/ _apoc2_track 8.0)) :!class /Script/Engine.MaterialInstanceDynamic)
      (Rendering|Material|SetScalarParameterValue (Variables|Default|GetLightGeyserGlowMat) "OpacOffset" (- 1.5 (/ _apoc2_track 8.0)) :!class /Script/Engine.MaterialInstanceDynamic)
      (Effects|Components|ParticleSystem|SetFloatParameter (Variables|Default|GetParts_Beam) "GeyserSpeed" (* _apoc2_track 0.5))
      (Game|Feedback|ClientStartCameraShake (Game|GetPlayerController 0) "/Game/myVFX/Apocalypse/shake_2.shake_2_C" (* (/ 1.0 (Transformation|GetDistanceTo (Game|Player|GetPlayerPawn 0))) 5e+02) "CameraLocal" "0, 0, 0")
      (Effects|Components|ParticleSystem|SetFloatParameter (Variables|Components|GetParts_Bubs) "BubbleSpawn" (* (- 1.0 _apoc2_track) 5e+01)))))

(event Custom|Stage1
  (Audio|SpawnSoundatLocation "/Game/myVFX/Apocalypse/Rumbling.Rumbling" (Transformation|GetWorldLocation (Variables|Default|GetDefaultSceneRoot)) "0, 0, 0" 1.0 1.0 0.0 0 0)
  (bind _bubbliness (Timeline|Stage1_TL Play)
    (:Update
      (Effects|Components|ParticleSystem|SetFloatParameter (Variables|Components|GetParts_Bubs) "BubbleSpawn" (* _bubbliness 5e+01))
      (Rendering|Material|SetScalarParameterValue (Variables|Default|GetSundialWaterMat) "Glowiness" (* _bubbliness 2.0) :!class /Script/Engine.MaterialInstanceDynamic))))

(event Custom|Stage3
  (bind (_direction _beamheight _newtrack_0) (Timeline|Stage3_TL Play)
    (:Update
      (Rendering|Material|SetScalarParameterValue (Variables|Default|GetBeamMat) "OpacOffset" (+ (* _beamheight -6.0) 1.25) :!class /Script/Engine.MaterialInstanceDynamic)
      (Rendering|Material|SetScalarParameterValue (Variables|Default|GetLightGeyserInnerMat) "OpacOffset" (+ (* _beamheight -6.0) 1.25) :!class /Script/Engine.MaterialInstanceDynamic)
      (Rendering|Material|SetScalarParameterValue (Variables|Default|GetLightGeyserInnerMat) "Brightness" (* _newtrack_0 2e+02) :!class /Script/Engine.MaterialInstanceDynamic)
      (Rendering|Material|SetScalarParameterValue (Variables|Default|GetLightGeyserGlowMat) "OpacOffset" (+ (* _beamheight -6.0) 1.25) :!class /Script/Engine.MaterialInstanceDynamic)
      (Effects|Components|ParticleSystem|SetFloatParameter (Variables|Default|GetParts_Beam) "GeyserSpeed" (+ (* _beamheight 4.0) 0.5))
      (Transformation|SetRelativeScale3D (Variables|Default|GetLightBeamInner) (Math|Vector|MakeVector (+ (* _beamheight 8.0) 1.2) (+ (* _beamheight 8.0) 1.2) 2e+02)))))

(event Custom|ConnectToSundial
  (bind _outactors (Actor|GetAllActorsOfClass "/Game/myVFX/Apocalypse/apocManager.apocManager_C"))
  (for _array_element _outactors
    (EventDispatchers|BindEventtoApocStage0 _array_element (delegate Custom|Stage0))
    (EventDispatchers|BindEventtoApocStage1 _array_element (delegate Custom|Stage1))
    (EventDispatchers|BindEventtoApocStage2 _array_element (delegate Custom|Stage2))
    (EventDispatchers|BindEventtoApocStage3 _array_element (delegate Custom|Stage3))))

(event EventBeginPlay
  (bind _returnvalue (Rendering|Material|CreateDynamicMaterialInstance "/Game/myVFX/Apocalypse/SundialMat.SundialMat" "None" "None" :!class /Script/Engine.KismetMaterialLibrary))
  (bind _output_get (Variables|Default|SetSundialMat _returnvalue))
  (Rendering|Material|SetMaterial (Variables|Default|GetStaticMesh) 0 _output_get)
  (bind _returnvalue_2 (Rendering|Material|CreateDynamicMaterialInstance "/Game/myVFX/Apocalypse/SundialWater.SundialWater" "None" "None" :!class /Script/Engine.KismetMaterialLibrary))
  (bind _output_get_2 (Variables|Default|SetSundialWaterMat _returnvalue_2))
  (Rendering|Material|SetMaterial (Variables|Default|GetStaticMesh) 1 _output_get_2)
  (bind _returnvalue_3 (Rendering|Material|CreateDynamicMaterialInstance "/Game/myVFX/Apocalypse/InnerBeamMat.InnerBeamMat" "None" "None" :!class /Script/Engine.KismetMaterialLibrary))
  (bind _output_get_3 (Variables|Default|SetLightGeyserInnerMat _returnvalue_3))
  (Rendering|Material|SetMaterial (Variables|Default|GetLightBeamInner) 0 _output_get_3)
  (bind _returnvalue_4 (Rendering|Material|CreateDynamicMaterialInstance "/Game/myVFX/Apocalypse/LightGeyserGlow.LightGeyserGlow" "None" "None" :!class /Script/Engine.KismetMaterialLibrary))
  (bind _output_get_4 (Variables|Default|SetLightGeyserGlowMat _returnvalue_4))
  (Rendering|Material|SetMaterial (Variables|Default|GetLightBeamWaterGlow) 0 _output_get_4)
  (bind _returnvalue_5 (Rendering|Material|CreateDynamicMaterialInstance "/Game/myVFX/Apocalypse/LightBeamMat.LightBeamMat" "None" "None" :!class /Script/Engine.KismetMaterialLibrary))
  (bind _output_get_5 (Variables|Default|SetBeamMat _returnvalue_5))
  (Rendering|Material|SetMaterial (Variables|Default|GetLightBeamWater) 0 _output_get_5)
  (Utilities|FlowControl|Delay 1.0)
  (bind _returnvalue_6 (Actor|GetActorOfClass "/Game/WorldScripts/Ocean2_Blueprint.Ocean2_Blueprint_C"))
  (Utilities|IsValid _returnvalue_6
    (:Is%20Valid
      (EventDispatchers|BindEventtoBindApocalpyse _returnvalue_6 (delegate Custom|ConnectToSundial)))))

(fn ConstructionScript)