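; Player character Blueprint that handles weapon spawning, health and pause UI, death, and Ink-driven NPC dialogue.
; Death ragdolls the mesh, drops the weapon and fades the camera before reporting the death, as does falling out of the world.
; Inputs drive dialogue choices, gamepad detection, pausing and debug-style level save/load.
; Native hooks access Ink variables on the locked NPC through casts, with dodge-count writes also updating NPC moods.
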(event OnComponentBeginOverlap(AIDetectionRange)
  (params (OverlappedComponent :type Primitive%20Component%20Object%20Reference) (OtherActor :type Actor%20Object%20Reference) (OtherComp :type Primitive%20Component%20Object%20Reference) (OtherBodyIndex :type Integer) (bFromSweep :type Boolean) (SweepResult :type Hit%20Result%20Structure%20%28by%20ref%29)))

(event OnComponentEndOverlap(AIDetectionRange)
  (params (OverlappedComponent :type Primitive%20Component%20Object%20Reference) (OtherActor :type Actor%20Object%20Reference) (OtherComp :type Primitive%20Component%20Object%20Reference) (OtherBodyIndex :type Integer))
  (bind _dialoguesystem (CallFunction|CastNPCs OtherActor))
  (Utilities|IsValid _dialoguesystem
    (:Is%20Valid
      (Default|InterruptStory _dialoguesystem))))

(event Custom|OnDestroyed_Event_0
  (params (DestroyedActor :type Actor%20Object%20Reference))
  (if (< (.z (Transformation|GetActorLocation DestroyedActor)) -1e+03)
    (Default|CallPlayerDied)))

(event EventBeginPlay
  (Game|AssignOnDestroyed (delegate Custom|OnDestroyed_Event_0))
  (bind _returnvalue (UserInterface|CreateWidget "/Game/HUD/PauseMenuWidget.PauseMenuWidget_C"))
  (Variables|Default|SetPauseMenuWidget _returnvalue)
  (bind _returnvalue_2 (UserInterface|CreateWidget "/Game/HUD/HealthBar.HealthBar_C"))
  (UserInterface|Viewport|AddtoViewport _returnvalue_2 1)
  (bind _returnvalue_3 (Game|SpawnActorfromClass "/Game/PrototypeCharacter/CharacterWeapon.CharacterWeapon_C" (Math|Transform|MakeTransform "0, 0, 0") "Undefined" 0 0 0))
  (Variables|Default|Setweapon _returnvalue_3)
  (Transformation|AttachComponentToComponent (Variables|Default|Getweapon) (Variables|Default|GetAnimMesh) "LeftHandSocket" "KeepRelative" "KeepRelative" "KeepWorld" true))

(event EventRagdollModel
  (bind _animmesh (Variables|Default|GetAnimMesh))
  (bind _bodycollision (Variables|Default|GetBodyCollision))
  (bind _deathcamerafadeouttime (Variables|Default|GetDeathCameraFadeoutTime))
  (Physics|SetSimulatePhysics _bodycollision false)
  (Collision|SetCollisionEnabled _bodycollision "NoCollision")
  (Physics|SetSimulatePhysics _animmesh true)
  (if (Variables|Default|GetinWater)
    (Physics|SetEnableGravity (Variables|Default|GetAnimMesh) false))
  (Collision|SetCollisionEnabled _animmesh "QueryAndPhysics")
  (Collision|SetCollisionObjectType _animmesh "ECC_Destructible")
  (bind _ascharacter_weapon (Utilities|Casting|CastToCharacterWeapon (Variables|Default|GetWeapon)))
  (Transformation|DetachFromActor _ascharacter_weapon "KeepWorld" "KeepWorld" "KeepWorld")
  (Collision|SetCollisionEnabled (Variables|/Game/PrototypeCharacter/CharacterWeapon.CharacterWeapon_C|GetWeaponModel _ascharacter_weapon) "QueryAndPhysics")
  (Physics|SetSimulatePhysics (Variables|/Game/PrototypeCharacter/CharacterWeapon.CharacterWeapon_C|GetWeaponModel _ascharacter_weapon) true)
  (CameraFades|StartCameraFade :self (Game|GetPlayerCameraManager 0) :ToAlpha 1.0 :Duration _deathcamerafadeouttime :bShouldFadeAudio true :bHoldWhenFinished true)
  (Utilities|FlowControl|Delay (+ _deathcamerafadeouttime 2.0))
  (Default|CallPlayerDied))

(event EventTick
  (params (DeltaSeconds :type Float%20%28single-precision%29)))

(event EventNativeSetDialogueInt
  (params (name :type String) (value :type Integer))
  (bind _lockedobject (Variables|Default|GetlockedObject))
  (bind _astown_guard (Utilities|Casting|CastToTownGuard _lockedobject)
    (:then
      (bind _asdialogue_system_bp (Utilities|Casting|CastToDialogueSystemBP (UserInterface|GetWidget (Variables|/Game/AICharacters/TownGuard/TownGuard.TownGuard_C|GetDialogueWidget _astown_guard))))
      (Utilities|IsValid _asdialogue_system_bp
        (:Is%20Valid
          (Default|SetInkVariableInt _asdialogue_system_bp name value)
          (if (Utilities|Enum|Equal(Enum) name "COUNT_playerDodges")
            (Default|SetAllMoodVariablesfromSource _astown_guard "NewEnumerator2")))))
    (:CastFailed
      (bind _asbaby (Utilities|Casting|CastToBaby _lockedobject)
        (:then
          (bind _asdialogue_system_bp_2 (Utilities|Casting|CastToDialogueSystemBP (UserInterface|GetWidget (Variables|/Game/AICharacters/Baby/Baby.Baby_C|GetDialogueWidget _asbaby))))
          (Utilities|IsValid _asdialogue_system_bp_2
            (:Is%20Valid
              (Default|SetInkVariableInt _asdialogue_system_bp_2 name value)
              (if (Utilities|Enum|Equal(Enum) name "COUNT_playerDodges")
                (Default|SetAllMoodVariablesfromSource _asbaby "NewEnumerator2")))))
        (:CastFailed
          (bind _asspellcaster (Utilities|Casting|CastToSpellcaster _lockedobject)
            (:then
              (bind _asdialogue_system_bp_3 (Utilities|Casting|CastToDialogueSystemBP (UserInterface|GetWidget (Variables|/Game/AICharacters/Spellcaster/Spellcaster.Spellcaster_C|GetDialogueWidget _asspellcaster))))
              (Utilities|IsValid _asdialogue_system_bp_3
                (:Is%20Valid
                  (Default|SetInkVariableInt _asdialogue_system_bp_3 name value)
                  (if (Utilities|Enum|Equal(Enum) name "COUNT_playerDodges")
                    (Default|SetAllMoodVariablesfromSource _asspellcaster "NewEnumerator2")))))
            (:CastFailed
              (bind _asguard_captain (Utilities|Casting|CastToGuardCaptain _lockedobject))
              (bind _asdialogue_system_bp_4 (Utilities|Casting|CastToDialogueSystemBP (UserInterface|GetWidget (Variables|/Game/AICharacters/GuardCaptain/GuardCaptain.GuardCaptain_C|GetDialogueWidget _asguard_captain))))
              (Utilities|IsValid _asdialogue_system_bp_4
                (:Is%20Valid
                  (Default|SetInkVariableInt _asdialogue_system_bp_4 name value)
                  (if (Utilities|Enum|Equal(Enum) name "COUNT_playerDodges")
                    (Default|SetAllMoodVariablesfromSource _asguard_captain "NewEnumerator2")))))))))))

(event EventNativeSetDialogueStr
  (params (name :type String) (value :type String))
  (bind _dialoguesystem (CallFunction|CastNPCs (Variables|Default|GetlockedObject)))
  (Utilities|IsValid _dialoguesystem
    (:Is%20Valid
      (Default|SetInkVariableString _dialoguesystem name value))))

(event EventInteractBP
  (Development|PrintString "InteractBP")
  (if (not (not (Variables|Default|GetisTalking)))
    (Default|CallMakeDialogueChoice (Variables|Default|GetcurrentChoiceIndex))))

(event Input|ActionEvents|InputActionDialogueOption1
  (params (Key :type Key%20Structure :default "None"))
  (:Pressed
    (Default|CallMakeDialogueChoice)))

(event Input|ActionEvents|InputActionDialogueOption2
  (params (Key :type Key%20Structure :default "None"))
  (:Pressed
    (Default|CallMakeDialogueChoice 1)))

(event Input|ActionEvents|InputActionDialogueOption3
  (params (Key :type Key%20Structure :default "None"))
  (:Pressed
    (Default|CallMakeDialogueChoice 2)))

(event Input|ActionEvents|InputActionDialogueOption4
  (params (Key :type Key%20Structure :default "None"))
  (:Pressed
    (Default|CallMakeDialogueChoice 3)))

(event Input|ActionEvents|InputActionPause
  (params (Key :type Key%20Structure :default "None"))
  (bind _pausemenuwidget (Variables|Default|GetPauseMenuWidget))
  (:Pressed
    (if (Variables|/Script/PitchPrototype.PauseMenu|GetbIsPaused (Variables|Default|GetPauseMenuWidget))
      (Class|PauseMenu|UnpauseGame _pausemenuwidget)
      (else
        (Class|PauseMenu|PauseGame _pausemenuwidget)))))

(event Input|ActionEvents|InputActionDialogueOptionUp
  (params (Key :type Key%20Structure :default "None"))
  (:Pressed
    (Default|CallChangeDialogueChoice false)))

(event Input|ActionEvents|InputActionDialogueOptionDown
  (params (Key :type Key%20Structure :default "None"))
  (:Pressed
    (Default|CallChangeDialogueChoice true)))

(event Input|KeyboardEvents|3
  (params (Key :type Key%20Structure :default "None"))
  ;[1 1 1] Load Current Level
  (:Pressed
    (bind _returnvalue (SaveGame|DoesSaveGameExist (Variables|Default|GetSlot%20Name)))
    (if _returnvalue
      (bind _returnvalue_2 (SaveGame|LoadGamefromSlot (Variables|Default|GetSlot%20Name)))
      (bind _output_get (Variables|Default|SetSaverSubClass _returnvalue_2))
      (bind _assave_game_1 (Utilities|Casting|CastToSaveGame1 _output_get))
      (Game|OpenLevel(byName) (Utilities|String|StringToName (Variables|/Game/LevelRestore/SaveGame1.SaveGame1_C|GetLevelName _assave_game_1)))
      (else
        (Game|OpenLevel(byObjectReference) "/Game/Maps/MainMap.MainMap")))))

(event Input|KeyboardEvents|2
  (params (Key :type Key%20Structure :default "None"))
  ;[1 1 1] Save Current Level
  (:Pressed
    (bind _returnvalue (SaveGame|DoesSaveGameExist (Variables|Default|GetSlot%20Name)))
    (if _returnvalue
      (bind _returnvalue_2 (SaveGame|LoadGamefromSlot (Variables|Default|GetSlot%20Name)))
      (bind _output_get (Variables|Default|SetSaverSubClass _returnvalue_2))
      (bind _assave_game_1 (Utilities|Casting|CastToSaveGame1 _output_get))
      (bind _returnvalue_3 (Game|GetCurrentLevelName true))
      (Variables|/Game/LevelRestore/SaveGame1.SaveGame1_C|SetLevelName _assave_game_1 _returnvalue_3)
      (else
        (bind _returnvalue_4 (SaveGame|CreateSaveGameObject "/Game/LevelRestore/SaveGame1.SaveGame1_C"))
        (bind _output_get_2 (Variables|Default|SetSaverSubClass _returnvalue_4))
        (bind _assave_game_1_2 (Utilities|Casting|CastToSaveGame1 _output_get_2))
        (bind _returnvalue_5 (Game|GetCurrentLevelName true))
        (Variables|/Game/LevelRestore/SaveGame1.SaveGame1_C|SetLevelName _assave_game_1_2 _returnvalue_5)))
    (SaveGame|SaveGametoSlot (Variables|Default|GetSaverSubClass) (Variables|Default|GetSlot%20Name))))

(event Input|KeyboardEvents|AnyKey
  (params (Key :type Key%20Structure :default "None"))
  (bind _returnvalue (Class|KismetInputLibrary|KeyIsGamepadKey Key))
  (:Pressed
    (Default|CallUpdateControlType _returnvalue)
    (Variables|Default|SetusingGamepad _returnvalue)))

(fn ConstructionScript)

(fn NativeGetDialogueInt
  (params (name :type String))
  (bind _dialoguesystem (CallFunction|CastNPCs (Variables|Default|GetlockedObject)))
  (Utilities|IsValid _dialoguesystem
    (:Is%20Valid
      (bind _intreturned (Default|GetInkVariableInt _dialoguesystem name))
      (return _intreturned))))

(fn CastNPCs
  (params (Actor :type Actor%20Object%20Reference))
  (bind _asbase_aicharacter (Utilities|Casting|CastToBaseAICharacter Actor)
    (:then
      (bind _asdialogue_system_bp (Utilities|Casting|CastToDialogueSystemBP (Variables|/Script/PitchPrototype.BaseAICharacter|GetdialogueSystem _asbase_aicharacter)))
      (return _asdialogue_system_bp))
    (:CastFailed
      (bind _asprop_npc (Utilities|Casting|CastToPropNPC Actor))
      (bind _asdialogue_system_bp_2 (Utilities|Casting|CastToDialogueSystemBP (UserInterface|GetWidget (Variables|/Game/DialogueSystem/PropNPC.PropNPC_C|GetDialogueWidget _asprop_npc))))
      (return _asdialogue_system_bp_2))))