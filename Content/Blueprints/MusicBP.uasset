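; Music manager actor that starts the Calm_BGM FMOD event on BeginPlay and keeps the event instance.
; It applies the Tides game instance's saved Master, SFX and Music volumes through VCA calls and binds to its change events for live updates.
; B and C keys switch the BGM's GameState parameter between high and zero with debug prints, apparently for testing adaptive music.
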(event Custom|MasterVolume
  (params (NewVolume :type Float%20%28single-precision%29))
  (Class|FMODBlueprintStatics|VCASetVolume "/Game/FMOD/VCAs/Master.Master" NewVolume))

(event Custom|SFXVolume
  (params (NewVolume :type Float%20%28single-precision%29))
  (Class|FMODBlueprintStatics|VCASetVolume "/Game/FMOD/VCAs/SFX.SFX" NewVolume))

(event Custom|MusicVolume
  (params (NewVolume :type Float%20%28single-precision%29))
  (Class|FMODBlueprintStatics|VCASetVolume 0 NewVolume))

(event EventBeginPlay
  (Input|EnableInput (Game|GetPlayerController 0))
  (bind _returnvalue (Class|FMODBlueprintStatics|PlayEvent2D "/Game/FMOD/Events/BGM/Calm_BGM.Calm_BGM"))
  (Variables|Default|SetBGMInstance _returnvalue)
  (bind _astides_game_instance_blueprint (Utilities|Casting|CastToTidesGameInstanceBlueprint (Game|GetGameInstance)))
  (EventDispatchers|BindEventtoOnMasterVolumeChanged _astides_game_instance_blueprint (delegate Custom|MasterVolume))
  (EventDispatchers|BindEventtoOnSFXVolumeChanged _astides_game_instance_blueprint (delegate Custom|SFXVolume))
  (EventDispatchers|BindEventtoOnMusicVolumeChanged _astides_game_instance_blueprint (delegate Custom|MusicVolume))
  (Class|FMODBlueprintStatics|VCASetVolume "/Game/FMOD/VCAs/Master.Master" (Variables|/Script/PitchPrototype.TidesGameInstance|GetMasterVolume _astides_game_instance_blueprint))
  (Class|FMODBlueprintStatics|VCASetVolume "/Game/FMOD/VCAs/SFX.SFX" (Variables|/Script/PitchPrototype.TidesGameInstance|GetSFXVolume _astides_game_instance_blueprint))
  (Class|FMODBlueprintStatics|VCASetVolume 0 (Variables|/Script/PitchPrototype.TidesGameInstance|GetMusicVolume _astides_game_instance_blueprint)))

(event EventTick
  (params (DeltaSeconds :type Float%20%28single-precision%29)))

(event Input|KeyboardEvents|B
  (params (Key :type Key%20Structure))
  (:Pressed
    (Class|FMODBlueprintStatics|EventInstanceSetParameter (Variables|Default|GetBGMInstance) "GameState" 0.95)
    (Development|PrintString "Gamestate; 1")))

(event Input|KeyboardEvents|C
  (params (Key :type Key%20Structure))
  (:Pressed
    (Class|FMODBlueprintStatics|EventInstanceSetParameter (Variables|Default|GetBGMInstance) "GameState" 0.0)
    (Development|PrintString "Gamestate; 0")))

(fn ConstructionScript)